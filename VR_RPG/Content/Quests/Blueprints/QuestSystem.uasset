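; QuestSystem is an actor that runs the current quest for the VR player.
; On BeginPlay it looks up the current quest in the Quests data table; for Reach Destination quests it reads location and trigger radius from Targets and spawns a waypoint there.
; Each tick it checks the VR character's 2D distance to that destination and, within range, destroys the waypoint and prints an arrival message.
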(event EventBeginPlay
  (bind _returnvalue (Utilities|GetDataTableRow "/Game/Quests/Blueprints/QuestStructure/Quests.Quests" (Utilities|String|StringToName (Utilities|String|ToString(Integer) (Variables|Default|GetCurrentQuest))))
    (:then
      (switch Utilities|FlowControl|Switch|SwitchonQuestTypes (.QuestType (Utilities|Struct|BreakQuestData _returnvalue))
        (:NewEnumerator1
          (bind _returnvalue_2 (Utilities|GetDataTableRow "/Game/Quests/Blueprints/QuestStructure/Targets.Targets" (Utilities|InttoName (.QuestID (Utilities|Struct|BreakQuestData _returnvalue))))
            (:then
              (bind _output_get (Variables|Default|SetDestination (.Location (Utilities|Struct|BreakReachDestination _returnvalue_2))))
              (Variables|Default|SetVariance (.VarianceTrigger (Utilities|Struct|BreakReachDestination _returnvalue_2)))
              (bind _returnvalue_3 (Game|SpawnActorfromClass "/Game/Quests/Blueprints/Waypoint.Waypoint_C" (Math|Transform|MakeTransform _output_get "0, 0, 0" "1,1,1") "Undefined" 0 0))
              (Variables|Default|SetActiveWaypoint _returnvalue_3))
            (:RowNotFound
              (Development|PrintString "Location For Quest Not Found"))))))
    (:RowNotFound
      (Development|PrintString "Quest Not Found"))))

(event Collision|EventActorBeginOverlap
  (params (OtherActor :type Actor%20Object%20Reference)))

(event EventTick
  (params (DeltaSeconds :type Float%20%28single-precision%29))
  (bind _activewaypoint (Variables|Default|GetActiveWaypoint))
  (bind _asvrcharacter (Utilities|Casting|CastToVRCharacter (Pawn|GetControlledPawn (Game|GetPlayerController 0))))
  (if (<= (Math|Vector|Distance2D(Vector) (Transformation|GetActorLocation _asvrcharacter) (Variables|Default|GetDestination)) (Variables|Default|GetVariance))
    (Utilities|IsValid _activewaypoint
      (:Is%20Valid
        (Actor|DestroyActor _activewaypoint)
        (Development|PrintString "Arrived At Location")))))

(fn ConstructionScript)