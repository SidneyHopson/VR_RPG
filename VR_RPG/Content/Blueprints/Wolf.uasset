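; Wolf enemy that wanders to random navmesh points until a forward line trace spots the VR player, then keeps chasing.
; Tick updates its health bar, repaths if the trace hits another wolf, and sets the anim instance's Bite flag when near the player.
; A looping timer applies damage while biting, using a random value also shown as its level.
; When the anim's Alive flag is false, it ragdolls and is destroyed.
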(event Custom|DamageEvent
  (bind _aswolf_anim (Utilities|Casting|CastToWolfAnim (Components|SkeletalMesh|GetAnimInstance (Variables|Character|GetMesh))))
  (if (Variables|/Game/Animations/WolfAnim.WolfAnim_C|GetBite _aswolf_anim)
    (bind _asvrcharacter (Utilities|Casting|CastToVRCharacter (Variables|Default|GetPlayer)))
    (bind _output_get (Variables|/Game/Blueprints/VRCharacter.VRCharacter_C|SetHealth _asvrcharacter (- (Variables|/Game/Blueprints/VRCharacter.VRCharacter_C|GetHealth _asvrcharacter) (Math|Conversions|ToFloat(Integer) (Variables|Default|GetDamage)))))
    (Development|PrintString (Utilities|String|ToString(Float) _output_get))))

(event EventBeginPlay
  (bind _output_get (Variables|Default|SetDamage (Math|Float|Round (Math|Random|RandomFloatinRange 1.0 1e+01))))
  (Rendering|Components|TextRender|SetText (Variables|Default|GetTextRender) (Utilities|Text|ToText(String) (Utilities|String|Append "Lv " (Utilities|String|ToString(Integer) _output_get) " Wolf")))
  (bind _returnvalue (Utilities|Time|SetTimerbyEvent (delegate Custom|DamageEvent) 2.0 true))
  (Variables|Default|SetNewVar_0 _returnvalue)
  (Variables|Default|SetTargetLocation (.RandomLocation (AI|Navigation|GetRandomReachablePointinRadius (Transformation|GetWorldLocation (Variables|Collision|GetCapsuleComponent)) 5e+04 0 0)))
  (AI|Navigation|SimpleMovetoLocation (AI|GetAIController self) (Variables|Default|GetTargetLocation)))

(event EventTick
  (params (DeltaSeconds :type Float%20%28single-precision%29))
  (bind _self self)
  (bind _capsulecomponent (Variables|Collision|GetCapsuleComponent))
  (bind _mesh (Variables|Character|GetMesh))
  (bind _returnvalue (AI|GetAIController _self))
  (bind _returnvalue_2 (Transformation|GetWorldLocation _capsulecomponent))
  (bind _returnvalue_3 (Components|SkeletalMesh|GetAnimInstance _mesh))
  (bind _ashealth_bar (Utilities|Casting|CastToHealthBar (UserInterface|GetUserWidgetObject (Variables|Default|GetWidget))))
  (Progress|SetPercent (Variables|/Game/Blueprints/HealthBar.HealthBar_C|GetProgressBar_322 _ashealth_bar) (/ (Variables|Default|GetHealth) (Variables|Default|GetMaxHealth)))
  (bind _aswolf_anim (Utilities|Casting|CastToWolfAnim (Components|SkeletalMesh|GetAnimInstance (Variables|Character|GetMesh))))
  (if (Variables|/Game/Animations/WolfAnim.WolfAnim_C|GetAlive _aswolf_anim)
    (bind _outhit (Collision|LineTraceByChannel _returnvalue_2 (+ _returnvalue_2 (* (Math|Vector|GetForwardVector (Transformation|GetWorldRotation _capsulecomponent)) 1.5e+03)) "TraceTypeQuery1" false 0 "ForOneFrame"))
    (bind _asvrcharacter (Utilities|Casting|CastToVRCharacter (.HitActor (Collision|BreakHitResult _outhit)))
      (:then
        (if (Variables|Default|GetSawPlayer)
          _
          (else
            _))
        (bind _output_get (Variables|Default|SetPlayer _asvrcharacter))
        (Variables|Default|SetSawPlayer true)
        (AI|Navigation|SimpleMovetoActor _returnvalue _output_get :!label _label)
        (if (<= (Math|Vector|Distance(Vector) (Transformation|GetActorLocation _output_get) (Transformation|GetWorldLocation (Variables|Collision|GetCapsuleComponent self))) 5e+02)
          (bind _aswolf_anim_2 (Utilities|Casting|CastToWolfAnim _returnvalue_3))
          (Variables|/Game/Animations/WolfAnim.WolfAnim_C|SetBite _aswolf_anim_2 true)
          (else
            (bind _aswolf_anim_3 (Utilities|Casting|CastToWolfAnim _returnvalue_3))
            (Variables|/Game/Animations/WolfAnim.WolfAnim_C|SetBite _aswolf_anim_3 false))))
      (:CastFailed
        (Utilities|Casting|CastToWolf (.HitActor (Collision|BreakHitResult _outhit))
          (:then
            (Variables|Default|SetTargetLocation (.RandomLocation (AI|Navigation|GetRandomReachablePointinRadius (Transformation|GetWorldLocation (Variables|Collision|GetCapsuleComponent)) 5e+04 0 0)))
            (AI|Navigation|SimpleMovetoLocation _returnvalue (Variables|Default|GetTargetLocation)))
          (:CastFailed
            (if (Variables|Default|GetSawPlayer)
              (goto _label)
              (else
                (if (<= (Math|Vector|Distance(Vector) (Transformation|GetWorldLocation (Variables|Collision|GetCapsuleComponent)) (Variables|Default|GetTargetLocation)) 5e+02)
                  (Variables|Default|SetTargetLocation (.RandomLocation (AI|Navigation|GetRandomReachablePointinRadius (Transformation|GetWorldLocation (Variables|Collision|GetCapsuleComponent)) 5e+04 0 0))))
                (AI|Navigation|SimpleMovetoLocation _returnvalue (Variables|Default|GetTargetLocation))))))))
    (else
      (Utilities|FlowControl|Delay 1.0)
      (Physics|SetSimulatePhysics (Variables|Character|GetMesh) true)
      (Utilities|FlowControl|Delay 0.9)
      (Actor|DestroyActor))))

(fn ConstructionScript)