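; Weapon is a VR pickup actor that can be held in either hand and used to strike enemies.
; Pickup turns off mesh physics and snaps the actor to the left or right hand socket based on the controller's name, while Drop restores physics and detaches it.
; Overlapping an Enemy calls Attack on the player's VRCharacter, passing the right controller if this is its right-hand attached actor, otherwise the left.
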(event EventBeginPlay)

(event EventTick
  (params (DeltaSeconds :type Float%20%28single-precision%29)))

(event EventPickupObject
  (params (AttachTo :type Scene%20Component%20Object%20Reference) (Hand :type Motion%20Controller%20Component%20Object%20Reference))
  (Physics|SetSimulatePhysics (Variables|Debug|GetStaticMeshComponent) false)
  (if (Utilities|Enum|Equal(Enum) (Utilities|GetObjectName Hand) "MotionController_L")
    (Transformation|AttachComponentToComponent (VehicleSound|GetRootComponent) AttachTo "hand_lSocket" "SnapToTarget" "SnapToTarget" "KeepWorld" false)
    (else
      (Transformation|AttachComponentToComponent (VehicleSound|GetRootComponent) AttachTo "hand_rSocket" "SnapToTarget" "SnapToTarget" "KeepWorld" false))))

(event Collision|EventActorBeginOverlap
  (params (OtherActor :type Actor%20Object%20Reference))
  (bind _asenemy (Utilities|Casting|CastToEnemy OtherActor))
  (bind _asvrcharacter (Utilities|Casting|CastToVRCharacter (Game|GetPlayerCharacter 0)))
  (if (== self (Variables|/Game/Blueprints/VRCharacter.VRCharacter_C|GetAttachedActor_R _asvrcharacter))
    (Default|Attack _asvrcharacter _asenemy (Variables|/Game/Blueprints/VRCharacter.VRCharacter_C|GetMotionController_R _asvrcharacter))
    (else
      (Default|Attack _asvrcharacter _asenemy (Variables|/Game/Blueprints/VRCharacter.VRCharacter_C|GetMotionController_L _asvrcharacter)))))

(event EventDrop
  (Physics|SetSimulatePhysics (Variables|Debug|GetStaticMeshComponent) true)
  (Transformation|DetachFromActor "KeepWorld" "KeepWorld" "KeepWorld"))

(fn ConstructionScript)