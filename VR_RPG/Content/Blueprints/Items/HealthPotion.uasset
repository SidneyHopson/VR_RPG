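; Health potion item actor that restores the VR player's health when used.
; UseItem casts the first player character to VRCharacter and adds HealVal to its Health, capped at MaxHealth.
; It then removes itself from the character's Items, refreshes the wrist menu's item display and destroys the actor.
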(event EventBeginPlay
  (|CallParentFunction) ; This node is disabled and will not be called.\nDrag off pins to build functionality.
)

(event Collision|EventActorBeginOverlap
  (params (OtherActor :type Actor%20Object%20Reference))
  (|CallParentFunction OtherActor) ; This node is disabled and will not be called.\nDrag off pins to build functionality.
)

(event EventTick
  (params (DeltaSeconds :type Float%20%28single-precision%29))
  (|CallParentFunction DeltaSeconds) ; This node is disabled and will not be called.\nDrag off pins to build functionality.
)

(event EventUseItem
  (bind _asvrcharacter (Utilities|Casting|CastToVRCharacter (Game|GetPlayerCharacter 0)))
  (if (> (+ (Variables|/Game/Blueprints/VRCharacter.VRCharacter_C|GetHealth _asvrcharacter) (Variables|Default|GetHeal%20Val)) (Variables|/Game/Blueprints/VRCharacter.VRCharacter_C|GetMaxHealth _asvrcharacter))
    (Variables|/Game/Blueprints/VRCharacter.VRCharacter_C|SetHealth _asvrcharacter (Variables|/Game/Blueprints/VRCharacter.VRCharacter_C|GetMaxHealth _asvrcharacter))
    (else
      (Variables|/Game/Blueprints/VRCharacter.VRCharacter_C|SetHealth _asvrcharacter (+ (Variables|/Game/Blueprints/VRCharacter.VRCharacter_C|GetHealth _asvrcharacter) (Variables|Default|GetHeal%20Val)))))
  (Utilities|Array|RemoveItem (Variables|/Game/Blueprints/VRCharacter.VRCharacter_C|GetItems _asvrcharacter) self)
  (Default|UpdateItems (Variables|/Game/Blueprints/VRCharacter.VRCharacter_C|GetWristMenuRef _asvrcharacter) (Variables|/Game/Blueprints/VRCharacter.VRCharacter_C|GetItems _asvrcharacter))
  (Actor|DestroyActor))

(fn ConstructionScript
  (|CallParentFunction))