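; Defense elixir item that temporarily boosts the player's resistance when used.
; UseItem casts player 0 to VRCharacter and raises its Resistance by a percentage of the current value.
; After a fixed delay on the item itself, it calls DecreaseResistance with IncreaseAmount to end the buff.
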(event EventBeginPlay
  (|CallParentFunction) ; This node is disabled and will not be called.\nDrag off pins to build functionality.
)

(event Collision|EventActorBeginOverlap
  (params (OtherActor :type Actor%20Object%20Reference))
  (|CallParentFunction OtherActor) ; This node is disabled and will not be called.\nDrag off pins to build functionality.
)

(event EventTick
  (params (DeltaSeconds :type Float%20%28single-precision%29))
  (|CallParentFunction DeltaSeconds) ; This node is disabled and will not be called.\nDrag off pins to build functionality.
)

(event EventUseItem
  (bind _asvrcharacter (Utilities|Casting|CastToVRCharacter (Game|GetPlayerCharacter 0)))
  (bind _output_get (Variables|Default|SetIncreaseAmount (* (Variables|/Game/Blueprints/VRCharacter.VRCharacter_C|GetResistance _asvrcharacter) 0.15)))
  (Default|IncreaseResistance _asvrcharacter _output_get)
  (Utilities|FlowControl|Delay 3e+01)
  (Default|DecreaseResistance _asvrcharacter _output_get))

(fn ConstructionScript
  (|CallParentFunction))