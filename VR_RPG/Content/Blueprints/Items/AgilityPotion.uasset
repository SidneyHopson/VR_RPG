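; Agility potion item that, when used, applies a timed agility effect to the player's VRCharacter.
; UseItem computes a fifth of current Agility, removes the potion from Items and refreshes the wrist menu.
; It calls IncreaseAgility with zero rather than the computed amount, waits a minute, decreases Agility by that amount, then destroys itself.
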(event EventBeginPlay
  (|CallParentFunction) ; This node is disabled and will not be called.\nDrag off pins to build functionality.
)

(event Collision|EventActorBeginOverlap
  (params (OtherActor :type Actor%20Object%20Reference))
  (|CallParentFunction OtherActor) ; This node is disabled and will not be called.\nDrag off pins to build functionality.
)

(event EventTick
  (params (DeltaSeconds :type Float%20%28single-precision%29))
  (|CallParentFunction DeltaSeconds) ; This node is disabled and will not be called.\nDrag off pins to build functionality.
)

(event EventUseItem
  (bind _asvrcharacter (Utilities|Casting|CastToVRCharacter (Game|GetPlayerCharacter 0)))
  (Variables|Default|SetIncreaseAMount' (* (Variables|/Game/Blueprints/VRCharacter.VRCharacter_C|GetAgility _asvrcharacter) 0.2))
  (Utilities|Array|RemoveItem (Variables|/Game/Blueprints/VRCharacter.VRCharacter_C|GetItems _asvrcharacter) self)
  (Default|UpdateItems (Variables|/Game/Blueprints/VRCharacter.VRCharacter_C|GetWristMenuRef _asvrcharacter) (Variables|/Game/Blueprints/VRCharacter.VRCharacter_C|GetItems _asvrcharacter))
  (Default|IncreaseAgility _asvrcharacter 0.0)
  (Utilities|FlowControl|Delay 6e+01)
  (Default|DecreaseAgility _asvrcharacter (Variables|Default|GetIncreaseAMount'))
  (Actor|DestroyActor))

(fn ConstructionScript
  (|CallParentFunction))