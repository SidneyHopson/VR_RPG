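; Item is a VR pickup actor that can be held in either hand, dropped, or stored in the inventory.
; Its construction script takes the mesh from PickupItemStruct.
; PickupObject stops physics and snaps the item to a left or right hand socket, chosen by motion controller name, while Drop detaches it and restores physics.
; AddToInventory attaches it to the player character, hidden, without collision or physics.
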(event EventBeginPlay)

(event Collision|EventActorBeginOverlap
  (params (OtherActor :type Actor%20Object%20Reference)))

(event EventTick
  (params (DeltaSeconds :type Float%20%28single-precision%29)))

(event EventPickupObject
  (params (AttachTo :type Scene%20Component%20Object%20Reference) (Hand :type Motion%20Controller%20Component%20Object%20Reference))
  (Physics|SetSimulatePhysics (Variables|Default|GetStaticMesh) false)
  (if (Utilities|Enum|Equal(Enum) (Utilities|GetObjectName Hand) "MotionController_L")
    (Transformation|AttachComponentToComponent (VehicleSound|GetRootComponent) AttachTo "hand_lSocket" "SnapToTarget" "SnapToTarget" "KeepWorld" false)
    (else
      (Transformation|AttachComponentToComponent (VehicleSound|GetRootComponent) AttachTo "hand_rSocket" "SnapToTarget" "SnapToTarget" "KeepWorld" false))))

(event EventDrop
  (Physics|SetSimulatePhysics (Variables|Default|GetStaticMesh) true)
  (Transformation|DetachFromActor "KeepWorld" "KeepWorld" "KeepWorld"))

(fn ConstructionScript
  (Components|StaticMesh|SetStaticMesh (Variables|Default|GetStaticMesh) (.staticmesh (Variables|Default|GetPickupItemStruct))))

(fn AddtoInventory
  (Transformation|AttachActorToActor (Game|GetPlayerCharacter 0) "None" "SnapToTarget" "SnapToTarget" "SnapToTarget" true)
  (Collision|SetCollisionEnabled (Variables|Default|GetStaticMesh) "NoCollision")
  (Physics|SetSimulatePhysics (Variables|Default|GetStaticMesh) false)
  (Rendering|SetVisibility (Variables|Default|GetStaticMesh) false true))