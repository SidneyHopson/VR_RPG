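; Background dragon pawn that wanders continuously by moving along a periodically re-randomized heading.
; A looping timer, its interval randomized once at BeginPlay, picks X and Y from random reachable navmesh points around CenterPoint, keeping the dragon's current Z.
; The look-at forward vector toward that target is stored in DesiredLocation, a direction despite its name.
; Tick feeds it into AddMovementInput, so the dragon never stops at a target.
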(event Custom|SetTargetLocation
  (bind _returnvalue (Transformation|GetActorLocation))
  (bind _radius (Variables|Default|GetRadius))
  (bind _centerpoint_ (Variables|Default|GetCenterPoint'))
  (bind _returnvalue_2 (Transformation|GetActorLocation _centerpoint_))
  (bind _randomlocation (AI|Navigation|GetRandomReachablePointinRadius _returnvalue_2 _radius 0 0))
  (Variables|Default|SetDesiredLocation (Math|Vector|GetForwardVector (Math|Rotator|FindLookatRotation _returnvalue (Math|Vector|MakeVector (.x _randomlocation) (.y _randomlocation) (.Z (Math|Vector|BreakVector _returnvalue)))))))

(event EventTick
  (params (DeltaSeconds :type Float%20%28single-precision%29))
  (Pawn|Input|AddMovementInput (Variables|Default|GetDesiredLocation) 1.0 false))

(event EventBeginPlay
  (Utilities|Time|SetTimerbyEvent (delegate Custom|SetTargetLocation) (Math|Random|RandomFloatinRange 1e+01 2e+01) true)
  (CallFunction|SetTargetLocation))

(fn ConstructionScript)