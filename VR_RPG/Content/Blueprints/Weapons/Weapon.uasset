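; Grabbable VR weapon actor that attacks enemies on overlap and can be broken and repaired.
; Pickup disables physics and snaps it to the left or right hand socket; drop detaches it and restores physics.
; Overlapping an Enemy calls the VRCharacter's Attack with the controller of the holding hand, defaulting to left.
; Break and Repair swap dirty materials and scale damage and sell price; Repair restores durability but leaves IsBroken true.
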(event EventBeginPlay)

(event EventTick
  (params (DeltaSeconds :type Float%20%28single-precision%29)))

(event EventPickupObject
  (params (AttachTo :type Scene%20Component%20Object%20Reference) (Hand :type Motion%20Controller%20Component%20Object%20Reference))
  ;[1 1 1] Pickup
  (Physics|SetSimulatePhysics (Variables|Debug|GetStaticMeshComponent) false)
  (if (Utilities|Enum|Equal(Enum) (Utilities|GetObjectName Hand) "MotionController_L")
    (Transformation|AttachComponentToComponent (VehicleSound|GetRootComponent) AttachTo "hand_lSocket" "SnapToTarget" "SnapToTarget" "KeepWorld" false)
    (else
      (Transformation|AttachComponentToComponent (VehicleSound|GetRootComponent) AttachTo "hand_rSocket" "SnapToTarget" "SnapToTarget" "KeepWorld" false))))

(event Collision|EventActorBeginOverlap
  (params (OtherActor :type Actor%20Object%20Reference))
  ;[1 1 1] Attack
  (bind _asenemy (Utilities|Casting|CastToEnemy OtherActor))
  (bind _asvrcharacter (Utilities|Casting|CastToVRCharacter (Game|GetPlayerCharacter 0)))
  (if (== self (Variables|/Game/Blueprints/VRCharacter.VRCharacter_C|GetAttachedActor_R _asvrcharacter))
    (Default|Attack _asvrcharacter _asenemy (Variables|/Game/Blueprints/VRCharacter.VRCharacter_C|GetMotionController_R _asvrcharacter))
    (else
      (Default|Attack _asvrcharacter _asenemy (Variables|/Game/Blueprints/VRCharacter.VRCharacter_C|GetMotionController_L _asvrcharacter)))))

(event EventDrop
  ;[1 1 1] Drop
  (Physics|SetSimulatePhysics (Variables|Debug|GetStaticMeshComponent) true)
  (Transformation|DetachFromActor "KeepWorld" "KeepWorld" "KeepWorld"))

(fn ConstructionScript)

(fn Break
  (bind _staticmeshcomponent (Variables|Debug|GetStaticMeshComponent))
  (if (not (Variables|Default|GetIsBroken))
    (Variables|Default|SetIsBroken true)
    (if (Utilities|Enum|Equal(Enum) (Utilities|GetDisplayName (Rendering|Material|GetMaterial (Variables|Debug|GetStaticMeshComponent) 0)) "M_WeaponSet_1")
      (Rendering|Material|SetMaterial _staticmeshcomponent 0 "/Game/Weapon_Pack/Materials/Weapons/M_WeaponSet_1Dirty.M_WeaponSet_1Dirty")
      (else
        (Rendering|Material|SetMaterial _staticmeshcomponent 0 "/Game/Weapon_Pack/Materials/Weapons/M_WeaponSet_2Dirty.M_WeaponSet_2Dirty")))
    (Variables|Default|SetDamage (* (Variables|Default|GetDamage) 0.25))
    (Variables|Default|SetSellPrice (/ (Variables|Default|GetSellPrice) 2))))

(fn Repair
  (bind _staticmeshcomponent (Variables|Debug|GetStaticMeshComponent))
  (bind _staticmeshcomponent_2 (Variables|Debug|GetStaticMeshComponent))
  (bind _returnvalue (Rendering|Material|GetMaterial _staticmeshcomponent 0))
  (bind _returnvalue_2 (Utilities|GetObjectName _returnvalue))
  (if (Variables|Default|GetIsBroken)
    (Variables|Default|SetIsBroken true)
    (Variables|Default|SetDurability (Variables|Default|GetMaxDurability))
    (if (Utilities|Enum|Equal(Enum) _returnvalue_2 "M_WeaponSet_1Dirty")
      (Rendering|Material|SetMaterial _staticmeshcomponent_2 0 "/Game/Weapon_Pack/Materials/Weapons/M_WeaponSet_1.M_WeaponSet_1")
      (Variables|Default|SetDamage (* (Variables|Default|GetDamage) 4.0) :!label _label)
      (Variables|Default|SetSellPrice (* (Variables|Default|GetSellPrice) 2))
      (elif (Utilities|Enum|Equal(Enum) _returnvalue_2 "M_WeaponSet_2Dirty")
        (Rendering|Material|SetMaterial _staticmeshcomponent_2 0 "/Game/Weapon_Pack/Materials/Weapons/M_WeaponSet_2.M_WeaponSet_2")
        (goto _label)))
    (else
      (Variables|Default|SetDurability (Variables|Default|GetMaxDurability)))))