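; VR shop actor that spawns a hammer, axe and sword as stock and flags the NPC's AnimBP when the VRCharacter enters or leaves ShopArea.
; SellCube destroys non-stock weapons still inside and simulating physics after two seconds, with no payout; other overlaps show help text.
; BuyCube routes stock items to BuyItem functions, which are empty stubs, and shows help text for anything else.
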(event OnComponentBeginOverlap(SellCube)
  (params (OverlappedComponent :type Primitive%20Component%20Object%20Reference) (OtherActor :type Actor%20Object%20Reference) (OtherComp :type Primitive%20Component%20Object%20Reference) (OtherBodyIndex :type Integer) (bFromSweep :type Boolean) (SweepResult :type Hit%20Result%20Structure%20%28by%20ref%29))
  ;[1 0 0] Sell
  (bind _asweapon (Utilities|Casting|CastToWeapon OtherActor)
    (:then
      (if (Math|Boolean|ORBoolean (== _asweapon (Variables|Default|GetItem1)) (== _asweapon (Variables|Default|GetItem2)) (== _asweapon (Variables|Default|GetItem3)))
        (Rendering|SetVisibility (Variables|Default|GetHelpText_S) true false :!label _label)
        (elif (Physics|IsSimulatingPhysics (Variables|/Script/Engine.StaticMeshActor|GetStaticMeshComponent _asweapon) "None")
          (Utilities|FlowControl|Delay 2.0)
          (if (and (Collision|IsOverlappingActor (Variables|Default|GetSell%20Cube) _asweapon :!class /Script/Engine.PrimitiveComponent) (Physics|IsSimulatingPhysics (Variables|/Script/Engine.StaticMeshActor|GetStaticMeshComponent _asweapon) "None"))
            (Actor|DestroyActor _asweapon)))))
    (:CastFailed
      (goto _label))))

(event OnComponentEndOverlap(SellCube)
  (params (OverlappedComponent :type Primitive%20Component%20Object%20Reference) (OtherActor :type Actor%20Object%20Reference) (OtherComp :type Primitive%20Component%20Object%20Reference) (OtherBodyIndex :type Integer))
  ;[1 0 0] Sell
  (Rendering|SetVisibility (Variables|Default|GetHelpText_S) false false))

(event OnComponentBeginOverlap(BuyCube)
  (params (OverlappedComponent :type Primitive%20Component%20Object%20Reference) (OtherActor :type Actor%20Object%20Reference) (OtherComp :type Primitive%20Component%20Object%20Reference) (OtherBodyIndex :type Integer) (bFromSweep :type Boolean) (SweepResult :type Hit%20Result%20Structure%20%28by%20ref%29))
  ;[0 1 0.1003] Buy\
  (if (== OtherActor (Variables|Default|GetItem1))
    (CallFunction|BuyItem1)
    (elif (== OtherActor (Variables|Default|GetItem2))
      (CallFunction|BuyItem2)
      (elif (== OtherActor (Variables|Default|GetItem3))
        (CallFunction|BuyItem3)
        (else
          (Rendering|SetVisibility (Variables|Default|GetHelpText_B) true false))))))

(event OnComponentBeginOverlap(ShopArea)
  (params (OverlappedComponent :type Primitive%20Component%20Object%20Reference) (OtherActor :type Actor%20Object%20Reference) (OtherComp :type Primitive%20Component%20Object%20Reference) (OtherBodyIndex :type Integer) (bFromSweep :type Boolean) (SweepResult :type Hit%20Result%20Structure%20%28by%20ref%29))
  ;[1 1 1] Interaction
  (Utilities|Casting|CastToVRCharacter OtherActor)
  (Variables|/Game/Blueprints/NPCs/ShopNPC_AnimBP.ShopNPC_AnimBP_C|SetIsPlayerClose? (Variables|Default|GetNPCANIM) true))

(event OnComponentEndOverlap(ShopArea)
  (params (OverlappedComponent :type Primitive%20Component%20Object%20Reference) (OtherActor :type Actor%20Object%20Reference) (OtherComp :type Primitive%20Component%20Object%20Reference) (OtherBodyIndex :type Integer))
  ;[1 1 1] Interaction
  (Utilities|Casting|CastToVRCharacter OtherActor)
  (Variables|/Game/Blueprints/NPCs/ShopNPC_AnimBP.ShopNPC_AnimBP_C|SetIsPlayerClose? (Variables|Default|GetNPCANIM) false))

(event OnComponentEndOverlap(BuyCube)
  (params (OverlappedComponent :type Primitive%20Component%20Object%20Reference) (OtherActor :type Actor%20Object%20Reference) (OtherComp :type Primitive%20Component%20Object%20Reference) (OtherBodyIndex :type Integer))
  ;[0 1 0.1003] Buy\
  (Rendering|SetVisibility (Variables|Default|GetHelpText_B) false false))

(event EventBeginPlay
  (CallFunction|SpawnItem1)
  (CallFunction|SpawnItem2)
  (CallFunction|SpawnItem3)
  (bind _asshop_npc_anim_bp (Utilities|Casting|CastToShopNPC_AnimBP (Components|SkeletalMesh|GetAnimInstance (Variables|/Script/Engine.Character|GetMesh (Variables|Default|GetShopNPC)))))
  (Variables|Default|SetNPCANIM _asshop_npc_anim_bp))

(event Collision|EventActorBeginOverlap
  (params (OtherActor :type Actor%20Object%20Reference)))

(event EventTick
  (params (DeltaSeconds :type Float%20%28single-precision%29)))

(fn ConstructionScript
  (Variables|Default|SetItem1_c "/Game/Blueprints/Weapons/Hammer.Hammer_C")
  (Variables|Default|SetItem2_c "/Game/Blueprints/Weapons/Axe.Axe_C")
  (Variables|Default|SetItem3_c "/Game/Blueprints/Weapons/Sword.Sword_C"))

(fn SpawnItem1
  (bind _returnvalue (Game|SpawnActorfromClass (Variables|Default|GetItem1_c) (Transformation|GetWorldTransform (Variables|Default|GetItem1Spawn)) "AdjustIfPossibleButAlwaysSpawn" 0 0))
  (Variables|Default|SetItem1 _returnvalue))

(fn SpawnItem2
  (bind _returnvalue (Game|SpawnActorfromClass (Variables|Default|GetItem2_c) (Transformation|GetWorldTransform (Variables|Default|GetItem2Spawn)) "AdjustIfPossibleButAlwaysSpawn" 0 0))
  (Variables|Default|SetItem2 _returnvalue))

(fn SpawnItem3
  (bind _returnvalue (Game|SpawnActorfromClass (Variables|Default|GetItem3_c) (Transformation|GetWorldTransform (Variables|Default|GetItem3Spawn)) "AdjustIfPossibleButAlwaysSpawn" 0 0))
  (Variables|Default|SetItem3 _returnvalue))

(fn BuyItem1)

(fn BuyItem2)

(fn BuyItem3)