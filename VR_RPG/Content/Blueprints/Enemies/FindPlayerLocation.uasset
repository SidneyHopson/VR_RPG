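; Behavior tree task for enemies that computes a move target near the player and writes it to a blackboard vector key.
; On execute, it casts the controlled pawn to Enemy and offsets the first player character's location backward along the enemy's forward vector by its AcceptanceRadius.
; The task then finishes successfully; a failed cast stops it without calling Finish Execute.
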(event EventReceiveExecuteAI
  (params (OwnerController :type AI%20Controller%20Object%20Reference) (ControlledPawn :type Pawn%20Object%20Reference))
  (bind _asenemy (Utilities|Casting|CastToEnemy ControlledPawn))
  (AI|BehaviorTree|SetBlackboardValueasVector (Variables|Default|GetVector) (+ (Transformation|GetActorLocation (Game|GetPlayerCharacter 0)) (* (Math|Vector|GetForwardVector (Transformation|GetActorRotation ControlledPawn)) (* (Variables|/Game/Blueprints/Enemies/Enemy.Enemy_C|GetAcceptanceRadius _asenemy) -1.0))))
  (AI|BehaviorTree|FinishExecute true))