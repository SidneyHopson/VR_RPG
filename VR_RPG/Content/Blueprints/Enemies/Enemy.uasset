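; Enemy Blueprint that shows a health bar and a name label and reports its alive state to AI.
; On BeginPlay it caches the EnemyStats widget from the Healthbar component.
; Each Tick it sets the progress bar from current over max health and writes the IsAlive blackboard key.
; The construction script builds the label from the name and truncated Damage, displayed as the level.
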(event EventBeginPlay
  (bind _asenemy_stats (Utilities|Casting|CastToEnemyStats (UserInterface|GetUserWidgetObject (Variables|Default|GetHealthbar))))
  (Variables|Default|SetEnemyStats _asenemy_stats))

(event EventTick
  (params (DeltaSeconds :type Float%20%28single-precision%29))
  (bind _returnvalue (AI|GetBlackboard 0))
  (bind _returnvalue_2 (Utilities|Name|MakeLiteralName "IsAlive"))
  (Progress|SetPercent (Variables|/Game/Blueprints/WIdgets/EnemyStats.EnemyStats_C|GetProgressBar_322 (Variables|Default|GetEnemyStats)) (/ (Variables|Default|GetCurrHealth) (Variables|Default|GetMaxHealth)))
  (if (<= (Variables|Default|GetCurrHealth) 0.0)
    (AI|Components|Blackboard|SetValueasBool _returnvalue _returnvalue_2 false)
    (else
      (AI|Components|Blackboard|SetValueasBool _returnvalue _returnvalue_2 true))))

(fn ConstructionScript
  (Rendering|Components|TextRender|SetText (Variables|Default|GetStats) (Utilities|Text|ToText(String) (Utilities|String|Append (Variables|Default|GetName) " - lvl " (Utilities|String|ToString(Integer) (Math|Float|Truncate (Variables|Default|GetDamage)))))))