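; Behavior tree task that drops loot from an AI-controlled enemy and rewards the player with gold.
; On a coin flip it spawns a Pickup_Blueprint at the pawn's transform, assigns a random ItemID and refreshes its display.
; Both outcomes then add random gold directly to the VRCharacter and finish successfully.
; If the player cast fails, the task never calls FinishExecute.
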(event EventReceiveExecuteAI
  (params (OwnerController :type AI%20Controller%20Object%20Reference) (ControlledPawn :type Pawn%20Object%20Reference))
  (switch int (Math|Random|RandomIntegerinRange 0 1)
    (:0
      (bind _returnvalue (Game|SpawnActorfromClass "/Game/Invenotry/Blueprints/Pickup_Blueprint.Pickup_Blueprint_C" (Transformation|GetActorTransform ControlledPawn) "AdjustIfPossibleButAlwaysSpawn" 0 0))
      (Variables|/Game/Invenotry/Blueprints/Pickup_Blueprint.Pickup_Blueprint_C|SetItemID _returnvalue (Math|Random|RandomIntegerinRange 1 10))
      (Default|UpdateDisplay _returnvalue))
    (:1
      _))
  (bind _asvrcharacter (Utilities|Casting|CastToVRCharacter (Game|GetPlayerCharacter 0)))
  (Variables|/Game/Blueprints/VRCharacter.VRCharacter_C|SetGoldAmount _asvrcharacter (+ (Variables|/Game/Blueprints/VRCharacter.VRCharacter_C|GetGoldAmount _asvrcharacter) (Math|Random|RandomIntegerinRange 10 60)))
  (AI|BehaviorTree|FinishExecute true))