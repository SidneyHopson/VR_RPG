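; Griffon enemy for a VR game that attacks the player in melee with its beak.
; The construction script sets its name and acceptance radius, then runs the parent's script.
; MeleeAttack snaps the Griffon to face the player and plays a moving attack montage.
; On the montage's notify, a short sphere trace from the Beak socket calls CalculateDamage if it hits the VRCharacter.
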(event EventBeginPlay
  (|CallParentFunction) ; This node is disabled and will not be called.\nDrag off pins to build functionality.
)

(event Collision|EventActorBeginOverlap
  (params (OtherActor :type Actor%20Object%20Reference)))

(event EventTick
  (params (DeltaSeconds :type Float%20%28single-precision%29))
  (|CallParentFunction DeltaSeconds) ; This node is disabled and will not be called.\nDrag off pins to build functionality.
)

(event EventMeleeAttack
  (bind _mesh (Variables|Character|GetMesh))
  (bind _returnvalue (Transformation|GetSocketTransform _mesh "Beak" "RTS_World"))
  (Transformation|SetActorRotation (Math|Rotator|FindLookatRotation (Transformation|GetActorLocation) (Transformation|GetActorLocation (Game|GetPlayerCharacter 0))))
  (Animation|Montage|PlayMontage (Variables|Character|GetMesh) "/Game/Animations/Griffon_MovingAttack.Griffon_MovingAttack"
    (:OnNotifyBegin
      (bind _outhit (Collision|SphereTraceByChannel (.location _returnvalue) (+ (.location _returnvalue) (* (Math|Vector|GetForwardVector (.rotation _returnvalue)) 1e+01)) 5e+01 "TraceTypeQuery1" false 0 "None"))
      (bind _asvrcharacter (Utilities|Casting|CastToVRCharacter (.hitactor _outhit)))
      (CallFunction|CalculateDamage _asvrcharacter))))

(fn ConstructionScript
  (Variables|Default|SetName "Griffon")
  (Variables|Default|SetAcceptanceRadius 2e+02)
  (|CallParentFunction))