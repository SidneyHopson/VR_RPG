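; Quest is an actor blueprint that carries a widget component showing a NewQuestScreen for the quest.
; On BeginPlay it casts the widget's user object to NewQuestScreen and hands it a reference to itself.
; An OrganizeQuestInEditor function teleports the quest to a spot slightly in front of and above the actor it is attached to.
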(event EventBeginPlay
  (bind _asnew_quest_screen (Utilities|Casting|CastToNewQuestScreen (UserInterface|GetUserWidgetObject (Variables|Default|GetWidget))))
  (Variables|/Game/Blueprints/Quests/NewQuestScreen.NewQuestScreen_C|SetQuest _asnew_quest_screen self))

(event Collision|EventActorBeginOverlap
  (params (OtherActor :type Actor%20Object%20Reference)))

(event EventTick
  (params (DeltaSeconds :type Float%20%28single-precision%29)))

(fn ConstructionScript)

(fn OrganizeQuestinEditor
  (bind _returnvalue (Actor|GetAttachParentActor))
  (Transformation|SetActorLocation (+ (Transformation|GetActorLocation _returnvalue) (* (Math|Vector|GetForwardVector (Transformation|GetActorRotation _returnvalue)) 2e+01) "0,0,100.000000") false true))