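; QuestBase is an Actor Blueprint that serves as a base for quests, holding a QuestInformation variable with the quest's data.
; Getter functions expose the quest name and description, plus a boolean for whether a linked quest exists, treating a LinkedQuestID of -1 as none.
; GetQuestID is an empty stub, and the event graph and construction script contain no logic.
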(event EventBeginPlay)

(event Collision|EventActorBeginOverlap
  (params (OtherActor :type Actor%20Object%20Reference)))

(event EventTick
  (params (DeltaSeconds :type Float%20%28single-precision%29)))

(fn ConstructionScript)

(fn GetQuestName
  (return (.QuestName (Utilities|Struct|BreakQuestData (Variables|Default|GetQuestInformation)))))

(fn GetQuestDescription
  (return (.QuestDescription (Utilities|Struct|BreakQuestData (Variables|Default|GetQuestInformation)))))

(fn GetLinkedQuest
  (return 0 (!= (.LinkedQuestID (Utilities|Struct|BreakQuestData (Variables|Default|GetQuestInformation))) -1)))

(fn GetQuestID)