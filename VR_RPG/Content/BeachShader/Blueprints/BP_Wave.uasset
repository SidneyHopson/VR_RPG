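; BP_Wave is a moving ocean wave actor that stamps a force material into a render target relative to a water mesh.
; Each tick fades strength in, draws the dynamic material at the wave's mesh-local position, and moves the actor along its yaw heading.
; Passing the end location, judged by distance from world origin, triggers a shore wash-up: strength fades, Y scale grows, and speed lerps toward reverse until the actor is destroyed.
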(event Custom|On%20Destroy
  (params (DeltaTime :type Float%20%28single-precision%29))
  (bind _returnvalue (Transformation|GetActorLocation))
  (bind _returnvalue_2 (* DeltaTime 1.0))
  (bind _waveendlocation (Variables|Default|GetWaveEndLocation))
  (bind _returnvalue_3 (Math|Vector|VectorLength _returnvalue))
  (bind _returnvalue_4 (Math|Vector|VectorLength _waveendlocation))
  ;[1 1 1] Shoreline Wash up effect and destroy
  (Utilities|FlowControl|Sequence
    (:then_0
      ;;[1 1 1] check if current location is less or greater than end location if triggered enable despawn
      (if (select (> (Math|Vector|VectorLength (Variables|Default|GetWaveStartLocation)) (Math|Vector|VectorLength (Variables|Default|GetWaveEndLocation))) (<= _returnvalue_3 _returnvalue_4) (>= _returnvalue_3 _returnvalue_4))
        (Variables|Default|SetisBeingDestroyed true)))
    (:then_1
      (if (Variables|Default|GetisBeingDestroyed)
        ;;[1 1 1] Check if wave strength is greater than 0, if so continue to shoreline code else destroy actor
        (if (> (Variables|Default|GetWaveStrInternal) 0.0)
          ;;[1 1 1] Reduce Wave Strength to show a fade out effect
          (Variables|Default|SetWaveStrInternal (- (Variables|Default|GetWaveStrInternal) (* DeltaTime 0.5)))
          ;;[1 1 1] Increase wave Y scale to increase shore wash up effect
          (Variables|Default|SetWaveScaleXY (Math|Vector2D|MakeVector2D (.x (Variables|Default|GetWaveScaleXY)) (+ (.y (Variables|Default|GetWaveScaleXY)) _returnvalue_2)))
          ;;[1 1 1] Lerp to an inverse current speed so we get a wash up on shore effect
          (Variables|Default|SetWaveSpeed (Math|Float|Lerp (Variables|Default|GetWaveSpeed) (* (Variables|Default|GetWaveSpeedInternal) -1.0) _returnvalue_2))
          (else
            (Actor|DestroyActor)))))))

(event Custom|Spawn%20Fade
  (params (DeltaTime :type Float%20%28single-precision%29))
  ;[1 1 1] Spawn Fade in: Start wave str at 0 so it will fade in, if at 0 add amount to internal str to fade in, once internal not less than input stop fade.
  (if (and (< (Variables|Default|GetWaveStrInternal) (Variables|Default|GetWaveStr)) (not (Variables|Default|GetisBeingDestroyed)))
    (Variables|Default|SetWaveStrInternal (+ (Variables|Default|GetWaveStrInternal) (* DeltaTime 0.25)))))

(event Custom|Wave%20Tick%20Params
  (params (DeltaTime :type Float%20%28single-precision%29))
  (bind _wavemarker (Variables|Default|GetWaveMarker))
  (bind _wavescalexy (Variables|Default|GetWaveScaleXY))
  ;[1 1 1] Update Wave Parameters and Wave Movement
  ;;[1 1 1] Update Wave Material instance input WaveScale: Make linear Color and Set input G (Y) to Wave Y Scale
  (Rendering|Material|SetVectorParameterValue _wavemarker "WaveScale" (Utilities|Struct|MakeLinearColor (.x _wavescalexy) (.y _wavescalexy) 0.0 0.0) :!class /Script/Engine.MaterialInstanceDynamic)
  ;;[1 1 1] Update Wave MI Force Strength Scalar to the internal Wave Str Variable
  (Rendering|Material|SetScalarParameterValue _wavemarker "ForceStrength" (Variables|Default|GetWaveStrInternal) :!class /Script/Engine.MaterialInstanceDynamic)
  ;;[1 1 1] Draw Material to wave render target reference
  (bind (_canvas _size _context) (Rendering|BeginDrawCanvastoRenderTarget (Variables|Default|GetWave_RenderTarget_Ref)))
  (bind (_screen_position _screen_size) (CallFunction|SetCanvasMaterialScaleandPosition _size (Math|Conversions|ToVector2D(Vector) (/ (Math|Transform|TransformLocation (Math|Transform|InvertTransform (Transformation|GetWorldTransform (Variables|Default|GetWaterMesh_ref))) (Transformation|GetActorLocation)) (Math|Float|MakeLiteralFloat 2.5e+04))) (/ (Variables|Default|GetWaveScale_Offset) (Variables|Default|GetWaveScale))))
  (Canvas|DrawMaterial _canvas _wavemarker _screen_position _screen_size "(X=0.000000,Y=0.000000)" "(X=1.000,Y=1.000)" (Variables|Default|GetRotation) "(X=0.500,Y=0.500)")
  (Rendering|EndDrawCanvastoRenderTarget _context)
  ;;[1 1 1] If the wave is not being destroyed update the actor location to the heading vector from the rotation angle
  (Transformation|SetActorLocation (- (Transformation|GetActorLocation) (* (Math|Vector|GetForwardVector (Math|Rotator|MakeRotator 0.0 0.0 (Variables|Default|GetRotation))) (* DeltaTime (Variables|Default|GetWaveSpeed)))) false false))

(event EventBeginPlay
  (bind _wavecollisionbox (Variables|Default|GetWaveCollisionBox))
  (bind _boxextent (Variables|/Script/Engine.BoxComponent|GetBoxExtent _wavecollisionbox))
  ;[1 1 1] Begin Play
  ;;[1 1 1] Set Start Location
  (Variables|Default|SetWaveStartLocation (Transformation|GetActorLocation))
  ;;[1 1 1] Create Wave Material Instance and store within reference
  (bind _returnvalue (Rendering|Material|CreateDynamicMaterialInstance "/Game/BeachShader/Materials/Effects/Wave_Mat.Wave_Mat" :!class /Script/Engine.KismetMaterialLibrary))
  (Variables|Default|SetWaveMarker _returnvalue)
  ;;[1 1 1] Set Wave Collision box to wave scale input
  (Components|Box|SetBoxExtent _wavecollisionbox (Math|Vector|MakeVector (.x _boxextent) (* (.y _boxextent) 0.0) (.z _boxextent)) true)
  ;;[1 1 1] Set Internal Speed to input wave speed
  (Variables|Default|SetWaveSpeedInternal (Variables|Default|GetWaveSpeed)))

(event EventTick
  (params (DeltaSeconds :type Float%20%28single-precision%29))
  ;[1 1 1] Update
  (Utilities|FlowControl|Sequence
    (:then_0
      (CallFunction|SpawnFade DeltaSeconds))
    (:then_1
      (CallFunction|WaveTickParams DeltaSeconds))
    (:then_2
      (CallFunction|OnDestroy DeltaSeconds))))

(fn ConstructionScript)