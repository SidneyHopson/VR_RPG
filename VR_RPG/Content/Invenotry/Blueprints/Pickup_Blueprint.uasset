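; A VR pickup actor that represents an inventory item and shows its image on two widget components.
; UpdateDisplay looks up ItemID in ItemsList and copies that item's image into both ItemDisplay widgets, from the Construction Script and on BeginPlay.
; PickupObject casts the attach component's owner to VRCharacter, adds the item to the InventoryWindow in its Inventory widget, then destroys the pickup.
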(event Custom|UpdateDisplay
  (bind _asitem_display (Utilities|Casting|CastToItemDisplay (UserInterface|GetUserWidgetObject (Variables|Default|GetWidget))))
  (Class|Image|SetBrush (Variables|/Game/Invenotry/Widgets/ItemDisplay.ItemDisplay_C|GetImage_59 _asitem_display) (Utilities|Struct|MakeSlateBrush (.ImageSize (Utilities|Struct|BreakSlateBrush (Variables|/Script/UMG.Image|GetBrush (Variables|/Game/Invenotry/Widgets/ItemDisplay.ItemDisplay_C|GetImage_59 _asitem_display)))) (.Margin (Utilities|Struct|BreakSlateBrush (Variables|/Script/UMG.Image|GetBrush (Variables|/Game/Invenotry/Widgets/ItemDisplay.ItemDisplay_C|GetImage_59 _asitem_display)))) (.TintColor (Utilities|Struct|BreakSlateBrush (Variables|/Script/UMG.Image|GetBrush (Variables|/Game/Invenotry/Widgets/ItemDisplay.ItemDisplay_C|GetImage_59 _asitem_display)))) (.ItemImage (Utilities|Struct|BreakItem (.Value (Utilities|Map|Find (Utilities|Struct|BreakItems (Variables|Default|GetItemsList)) (Variables|Default|GetItemID))))) (.DrawAs (Utilities|Struct|BreakSlateBrush (Variables|/Script/UMG.Image|GetBrush (Variables|/Game/Invenotry/Widgets/ItemDisplay.ItemDisplay_C|GetImage_59 _asitem_display)))) (.Tiling (Utilities|Struct|BreakSlateBrush (Variables|/Script/UMG.Image|GetBrush (Variables|/Game/Invenotry/Widgets/ItemDisplay.ItemDisplay_C|GetImage_59 _asitem_display)))) (.Mirroring (Utilities|Struct|BreakSlateBrush (Variables|/Script/UMG.Image|GetBrush (Variables|/Game/Invenotry/Widgets/ItemDisplay.ItemDisplay_C|GetImage_59 _asitem_display))))))
  (bind _asitem_display_2 (Utilities|Casting|CastToItemDisplay (UserInterface|GetUserWidgetObject (Variables|Default|GetWidget2))))
  (Class|Image|SetBrush (Variables|/Game/Invenotry/Widgets/ItemDisplay.ItemDisplay_C|GetImage_59 _asitem_display_2) (Variables|/Script/UMG.Image|GetBrush (Variables|/Game/Invenotry/Widgets/ItemDisplay.ItemDisplay_C|GetImage_59 _asitem_display))))

(event EventBeginPlay
  (CallFunction|UpdateDisplay))

(event Collision|EventActorBeginOverlap
  (params (OtherActor :type Actor%20Object%20Reference)))

(event EventTick
  (params (DeltaSeconds :type Float%20%28single-precision%29)))

(event EventPickupObject
  (params (AttachTo :type Scene%20Component%20Object%20Reference) (Hand :type Motion%20Controller%20Component%20Object%20Reference))
  (bind _asvrcharacter (Utilities|Casting|CastToVRCharacter (Components|GetOwner AttachTo)))
  (bind _asinventory (Utilities|Casting|CastToInventory (UserInterface|GetUserWidgetObject (Variables|/Game/Blueprints/VRCharacter.VRCharacter_C|GetInventoryWidget _asvrcharacter))))
  (Default|AddItem (Variables|/Game/Blueprints/WIdgets/Inventory.Inventory_C|GetInventoryWindow _asinventory) (.Value (Utilities|Map|Find (Utilities|Struct|BreakItems (Variables|Default|GetItemsList)) (Variables|Default|GetItemID))))
  (Actor|DestroyActor))

(fn ConstructionScript
  (CallFunction|UpdateDisplay))